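; Player actor that moves in a constant straight line and can fire bullets.
; BeginPlay sets the final velocity from the normalized player velocity scaled by an editable factor, and Tick applies it as an unswept local offset each frame, without delta-time scaling.
; DisparaBala spawns a BALA actor at the player's location, passing the given Normal as the bullet's velocity.
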(event EventTick
  (params (DeltaSeconds :type Float%20%28single-precision%29))
  (Transformation|AddActorLocalOffset (Variables|Default|GetVelocidadFinalPlayer) false false))

(event EventBeginPlay
  (Variables|Default|SetVelocidadFinalPlayer (* (Math|Vector|Normalize (Variables|Default|GetVelocidad%20Player)) (Variables|Default|GetFactor%20Editable))))

(fn ConstructionScript)

(fn DisparaBala
  (params (Normal :type Vector))
  (Game|SpawnActorfromClass "/Game/Blueprint/BALA.BALA_C" (Math|Transform|MakeTransform (Transformation|GetActorLocation) "0, 0, 0" "1.000000,1.000000,1.000000") "Undefined" "MultiplyWithRoot" 0 Normal 0))